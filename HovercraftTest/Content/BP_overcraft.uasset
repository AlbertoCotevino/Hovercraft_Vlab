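; Player-controlled hovercraft that moves a physics-driven Cube through forces and torque.
; One input axis pushes the Cube along its right vector by Speed, and the other applies mass-independent yaw torque scaled by Intensity.
; ReciveHoverPush takes a push from a hover component and applies it at that component's world location, so off-center pushes can tilt the craft.
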(event EventReciveHoverPush
  (params (Push :type Vector) (Hover_component :type BP%20Hover%20Component%20Object%20Reference))
  (Class|PrimitiveComponent|AddForceatLocation (Variables|Default|GetCube) Push (Transformation|GetWorldLocation Hover_component) "None"))

(event Input|AxisEvents|InputAxisControl
  (params (AxisValue :type Float%20%28single-precision%29))
  (bind _cube (Variables|Default|GetCube))
  (Physics|AddForce _cube (* (Math|Vector|GetRightVector _cube) (* AxisValue (Variables|Default|Getspeed))) "None" false))

(event Input|AxisEvents|InputAxiscontrol2
  (params (AxisValue :type Float%20%28single-precision%29))
  (Class|PrimitiveComponent|AddTorque (Variables|Default|GetCube) (Math|Vector|MakeVector 0.0 0.0 (* AxisValue (Variables|Default|Getintensity))) "None" true))

(fn ConstructionScript)