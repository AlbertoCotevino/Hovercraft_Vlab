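; BP_hoverComponent is a hover component that computes an upward or downward Z push for its owning actor.
; Each tick it line traces straight down from its world location over PropelDistance on the Visibility channel, with debug drawing.
; The hit time samples PowerScalingCurve to scale Power, without checking for a hit.
; It sends the push and itself to the owner through ReciveHoverPushMessage, leaving the owner to apply it.
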(event EventBeginPlay)

(event EventTick
  (params (DeltaSeconds :type Float%20%28single-precision%29))
  (bind (_start_point _end_point) (CallFunction|GetLInetraceStartEnd))
  (bind _outhit (Collision|LineTraceByChannel _start_point _end_point "TraceTypeQuery1" false 0 "ForOneFrame"))
  (Class|BPIHoverVeicle|ReciveHoverPush(Message) (Components|GetOwner) (Math|Vector|MakeVector 0.0 0.0 (Math|Float|Lerp 0.0 (Variables|Default|GetPower) (Math|Curves|GetFloatValue (Variables|Default|GetPowerScalingCurve) (.time _outhit)))) self))

(fn GetLInetraceStartEnd
  (return (Transformation|GetWorldLocation) (- (Transformation|GetWorldLocation) (Math|Vector|MakeVector 0.0 0.0 (Variables|Default|GetPropelDistance)))))